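; BP_TDGameMode is a tower defense game mode that holds wave, gold and lives state.
; BeginPlay initializes that state, then calls StartNewWave after a short delay.
; StartNewWave increments CurrentWave only when no wave is active, but initialization marks one active, and its EnemiesPerWave formula is unconnected.
; SpawnEnemy, OnEnemyReachedEnd, AddGold and RemoveLife are empty stubs.
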(event Custom|StartWave
  (CallFunction|StartNewWave))

(event EventBeginPlay
  (CallFunction|InitializeGameState) ; Sets initial Game Values
  (Utilities|FlowControl|Delay 1.0)
  (CallFunction|StartWave) ; Calls Event to Start New Wave
)

(fn ConstructionScript)

(fn InitializeGameState
  (Utilities|FlowControl|Sequence
    (:then_0
      (Variables|Default|SetCurrentWave 0))
    (:then_1
      (Variables|Default|SetPlayerGold 100))
    (:then_2
      (Variables|Default|SetPlayerLives 20))
    (:then_3
      (Variables|Default|SetIsWaveActive true))))

(fn StartNewWave
  (if (not (Variables|Default|GetIsWaveActive))
    (bind _result (Math|Integer|IncrementInt (Variables|Default|GetCurrentWave)))))

(fn SpawnEnemy)

(fn OnEnemyReachedEnd)

(fn AddGold)

(fn RemoveLife)